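; Sushi cookware Blueprint that displays its name and on-screen progress for cutting fish and rolling sushi.
; On BeginPlay it writes SushiName into its name widget.
; SpawnCuttingUI and SpawnRollingUI each reveal the shared progress widget, play their own timeline, then hide it.
; Timeline alpha fills the bar and scales CuttingTime or RollingTime into counting-up time text, without setting timeline length.
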(event EventBeginPlay
  (bind _aswbp_cookware_name (Utilities|Casting|CastToWBP_CookwareName (UserInterface|GetUserWidgetObject (Variables|Default|GetCookwareName))))
  (Rendering|Components|TextRender|SetText (Variables|/Game/Blueprints/UI/WBP_CookwareName.WBP_CookwareName_C|GetTextBlock_34 _aswbp_cookware_name) (Utilities|Text|ToText(Name) (Variables|Default|GetSushiName))))

(event EventSpawnCuttingUI
  (bind _aswbp_cookware_progress (Utilities|Casting|CastToWBP_CookwareProgress (UserInterface|GetUserWidgetObject (Variables|Default|GetWidget))))
  (Widget|SetVisibility (Variables|/Game/Blueprints/UI/WBP_CookwareProgress.WBP_CookwareProgress_C|GetProgressBar _aswbp_cookware_progress) "Visible")
  (bind _alpha (Timeline|CuttingTimeline Play)
    (:Update
      (Progress|SetPercent (Variables|/Game/Blueprints/UI/WBP_CookwareProgress.WBP_CookwareProgress_C|GetProgressBar _aswbp_cookware_progress) (Math|Float|Lerp 0.0 1.0 _alpha))
      (Rendering|Components|TextRender|SetText (Variables|/Game/Blueprints/UI/WBP_CookwareProgress.WBP_CookwareProgress_C|GetTimeText _aswbp_cookware_progress) (Utilities|Text|ToText(String) (Utilities|String|Append "Cutting Fish: " (Class|KismetStringLibrary|TimeSecondstoString (Math|Float|Lerp 0.0 (Variables|Default|GetCuttingTime) _alpha))))))
    (:Finished
      (Widget|SetVisibility (Variables|/Game/Blueprints/UI/WBP_CookwareProgress.WBP_CookwareProgress_C|GetTimeText _aswbp_cookware_progress) "Hidden"))))

(event EventSpawnRollingUI
  (bind _aswbp_cookware_progress (Utilities|Casting|CastToWBP_CookwareProgress (UserInterface|GetUserWidgetObject (Variables|Default|GetWidget))))
  (Widget|SetVisibility (Variables|/Game/Blueprints/UI/WBP_CookwareProgress.WBP_CookwareProgress_C|GetProgressBar _aswbp_cookware_progress) "Visible")
  (bind _alpha (Timeline|Timeline Play)
    (:Update
      (Progress|SetPercent (Variables|/Game/Blueprints/UI/WBP_CookwareProgress.WBP_CookwareProgress_C|GetProgressBar _aswbp_cookware_progress) (Math|Float|Lerp 0.0 1.0 _alpha))
      (Rendering|Components|TextRender|SetText (Variables|/Game/Blueprints/UI/WBP_CookwareProgress.WBP_CookwareProgress_C|GetTimeText _aswbp_cookware_progress) (Utilities|Text|ToText(String) (Utilities|String|Append "Rolling Sushi: " (Class|KismetStringLibrary|TimeSecondstoString (Math|Float|Lerp 0.0 (Variables|Default|GetRollingTime) _alpha))))))
    (:Finished
      (Widget|SetVisibility (Variables|/Game/Blueprints/UI/WBP_CookwareProgress.WBP_CookwareProgress_C|GetProgressBar _aswbp_cookware_progress) "Hidden"))))

(fn ConstructionScript)